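; SizeChanger is a Blueprint meant to resize table-and-chair actors from a UI_ChangeDimension widget, though its event wiring is disconnected.
; RefreshActor spawns a BP_TableWithChair at the given actor's transform with the new CurrWidth, destroys the original and returns the replacement.
; BeginPlay and ActorChange are empty; the widget setup and the code assigning the replacement to the widget's OBJOwner never run.
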(event `self.ReceiveBeginPlay`)

(event `ActorChange`
  (params (value :type Integer) (Owner :type "/Game/Blueprint/BP_TableWithChair Object Reference")))

(fn `Refresh Actor`
  (params (actor :type "/Game/Blueprint/BP_TableWithChair Object Reference") (Width :type Integer))
  (returns (newActor :type "/Game/Blueprint/BP_TableWithChair Object Reference"))
  (bind _returnvalue (`|SpawnActorFromClass` "/Game/Blueprint/BP_TableWithChair.BP_TableWithChair_C" (`Actor.GetTransform` actor) "Undefined" "MultiplyWithRoot" null Width null))
  (`Actor.K2_DestroyActor` actor)
  (return _returnvalue))