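; BP_TableWithChair is a clickable table actor that procedurally lays out a row of chairs to suit its width.
; The construction script derives the chair count from CurrWidth and spaces the chairs evenly along local Y, allowing for end margins.
; Each chair is added as an instance to InstancedChairs.
; On click, the actor passes itself to the player controller through ActorClickedMessage.
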(event `self.ReceiveBeginPlay`)

(event `self.ReceiveActorOnClicked`
  (params (ButtonPressed :type "Key Structure"))
  (message `/Game/Blueprint/sizeChanger.actorClicked` (`GameplayStatics.GetPlayerController` 0) self))

(fn `UserConstructionScript`
  (bind _nchairs (`self.nChairs`))
  (set `self.width` (`self.CurrWidth`))
  (set `self.nChairs` (/ (- (`self.width`) 60) 130))
  (bind _output_get (set `self.Distance` (/ (- (- (`self.width`) 120) (* 100 (`self.nChairs`))) (+ (`self.nChairs`) 1))))
  (for _index (range 1 (+ _nchairs 1))
    (if (!= _nchairs 0)
      (set `self.PreDistance` _output_get)
      (if (== _index 1)
        (set `self.PreDistance` (+ (`self.PreDistance`) 60)))
      (bind _output_get_2 (set `self.CurrPos` (+ (`self.CurrPos`) (`self.PreDistance`))))
      (`InstancedStaticMeshComponent.AddInstance` (`self.InstancedChairs`) (`KismetMathLibrary.MakeTransform` (`KismetMathLibrary.MakeVector` 0.0 _output_get_2)) false)
      (set `self.CurrPos` (+ (`self.CurrPos`) 100.0)))))