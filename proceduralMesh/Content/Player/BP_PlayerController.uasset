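; Player controller that lets the player resize a clicked table-with-chair actor through a dimension widget.
; ActorClicked creates a new UI_ChangeDimension seeded with the actor's width and binds to its size callback.
; ActorChange calls RefreshActor, which rebuilds by respawning BP_TableWithChair at the same transform with the new width and destroying the old actor.
; The widget's owner reference is then repointed to the replacement.
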(event `self.ReceiveBeginPlay`)

(event `/Game/Blueprint/SizeChanger.actorClicked`
  (params (beingClicked :type "/Game/Blueprint/BP_TableWithChair Object Reference"))
  (bind _returnvalue (`|CreateWidget` "/Game/UserInterface/UI_ChangeDimension.UI_ChangeDimension_C" self (`KismetMathLibrary.Conv_IntToDouble` (`Table.width` beingClicked)) beingClicked))
  (bind _output_get (set `self.dimensionWidget` _returnvalue))
  (`UserWidget.AddToViewport` _output_get 0)
  (`Widget.SetVisibility` _output_get "Visible")
  (add `/Game/UserInterface/UI_ChangeDimension.SizeCall` (`self.DimensionWidget`) (`|CreateDelegate` :!event `ActorChange`)))

(event `ActorChange`
  (params (value :type Integer) (Owner :type "/Game/Blueprint/BP_TableWithChair Object Reference"))
  (bind _newactor (`self.Refresh Actor` value Owner))
  (set `/Game/UserInterface/UI_ChangeDimension.OBJ_Owner` _newactor (`self.DimensionWidget`)))

(fn `Refresh Actor`
  (params (Width :type Integer) (actor :type "/Game/Blueprint/BP_TableWithChair Object Reference (by ref)"))
  (returns (newActor :type "/Game/Blueprint/BP_TableWithChair Object Reference"))
  (bind _returnvalue (`|SpawnActorFromClass` "/Game/Blueprint/BP_TableWithChair.BP_TableWithChair_C" (`self.GetTransform` actor) "Undefined" "MultiplyWithRoot" null Width null))
  (`self.K2_DestroyActor` actor)
  (return _returnvalue))

(fn `UserConstructionScript`)